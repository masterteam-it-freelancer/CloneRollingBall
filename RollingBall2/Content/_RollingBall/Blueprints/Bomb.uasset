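; Bomb pickup actor for the rolling ball game that detonates visually after the ball touches it.
; Overlap of PickupArea by RollingBallBP spawns a sound at world origin and starts a three-second delay, then emits a pulse ring at the mesh and destroys the actor.
; Leaving the area deactivates the sound but does not cancel the detonation.
; No damage or force is applied to the stored ball reference.
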(event `self.PickupArea.OnComponentBeginOverlap`
  (params (OverlappedComponent :type "PrimitiveComponent Object Reference") (OtherActor :type "Actor Object Reference") (OtherComp :type "PrimitiveComponent Object Reference") (OtherBodyIndex :type Integer) (bFromSweep :type Boolean) (SweepResult :type "HitResult Structure (by ref)"))
  (bind _asrolling_ball_bp (cast `/Game/_RollingBall/Blueprints/RollingBallBP` OtherActor))
  (set `self.Ball` _asrolling_ball_bp)
  (bind _returnvalue (`GameplayStatics.SpawnSoundAtLocation` (`self.Sound`) (0.0 0.0 0.0) (struct) 1.0 1.0 0.0 null null))
  (bind _output_get (set `self.ToSound` _returnvalue))
  (`ActorComponent.SetActive` _output_get true false)
  (`KismetSystemLibrary.Delay` 3.0)
  (if true
    (`GameplayStatics.SpawnEmitterAtLocation` "/Game/MaterialFunctionCollection/ShowcaseAssets/ExampleContent/Effects/P_Pulse_Ring.P_Pulse_Ring" (`SceneComponent.K2_GetComponentLocation` (`self.StaticMesh`)))
    (`KismetSystemLibrary.Delay` 0.2)
    (`self.K2_DestroyActor`)))

(event `self.PickupArea.OnComponentEndOverlap`
  (params (OverlappedComponent :type "PrimitiveComponent Object Reference") (OtherActor :type "Actor Object Reference") (OtherComp :type "PrimitiveComponent Object Reference") (OtherBodyIndex :type Integer))
  (cast `/Game/_RollingBall/Blueprints/RollingBallBP` OtherActor)
  (`ActorComponent.SetActive` (`self.ToSound`) false false))

(fn `UserConstructionScript`
  (`parent.UserConstructionScript`))