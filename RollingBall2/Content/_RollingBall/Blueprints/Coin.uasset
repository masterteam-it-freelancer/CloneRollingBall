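; Collectible coin for the rolling ball game that adds its Value to the RollingBallBP's Score and destroys itself after a short delay.
; An ObjectInfo widget receives a reference to the coin and starts hidden.
; PickupArea overlap plays a sound and particle and shows the widget, which end overlap also sets visible rather than hiding.
; A separate Sphere overlap handles the scoring and destruction.
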(event `self.ReceiveBeginPlay`
  (`parent.ReceiveBeginPlay`)
  (bind _asobject_info (cast `/Game/_RollingBall/Blueprints/ObjectInfo` (`WidgetComponent.GetUserWidgetObject` (`self.Widget`))))
  (set `/Game/_RollingBall/Blueprints/ObjectInfo.Coin` self _asobject_info)
  (`Widget.SetVisibility` _asobject_info "Hidden"))

(event `self.PickupArea.OnComponentBeginOverlap`
  (params (OverlappedComponent :type "PrimitiveComponent Object Reference") (OtherActor :type "Actor Object Reference") (OtherComp :type "PrimitiveComponent Object Reference") (OtherBodyIndex :type Integer) (bFromSweep :type Boolean) (SweepResult :type "HitResult Structure (by ref)"))
  ;[1 1 1] Play Sound and Particle for Coin
  (cast `/Game/_RollingBall/Blueprints/RollingBallBP` OtherActor)
  (`GameplayStatics.PlaySound2D` "/Game/ActionRPGStarterSystem/InventorySystem/JigSaw/Sounds/Cue_VendorSound1.Cue_VendorSound1" 1.0 1.0 0.0 null null)
  (`GameplayStatics.SpawnEmitterAtLocation` (`self.PickupParticle`) (`self.K2_GetActorLocation`) (struct) (1.0 1.0 1.0) false)
  (bind _asobject_info (cast `/Game/_RollingBall/Blueprints/ObjectInfo` (`WidgetComponent.GetUserWidgetObject` (`self.Widget`))))
  (`Widget.SetVisibility` _asobject_info "Visible"))

(event `self.PickupArea.OnComponentEndOverlap`
  (params (OverlappedComponent :type "PrimitiveComponent Object Reference") (OtherActor :type "Actor Object Reference") (OtherComp :type "PrimitiveComponent Object Reference") (OtherBodyIndex :type Integer))
  ;[1 1 1] Play Sound and Particle for Coin
  (cast `/Game/_RollingBall/Blueprints/RollingBallBP` OtherActor)
  (bind _asobject_info (cast `/Game/_RollingBall/Blueprints/ObjectInfo` (`WidgetComponent.GetUserWidgetObject` (`self.Widget`))))
  (`Widget.SetVisibility` _asobject_info "Visible"))

(event `self.Sphere.OnComponentBeginOverlap`
  (params (OverlappedComponent :type "PrimitiveComponent Object Reference") (OtherActor :type "Actor Object Reference") (OtherComp :type "PrimitiveComponent Object Reference") (OtherBodyIndex :type Integer) (bFromSweep :type Boolean) (SweepResult :type "HitResult Structure (by ref)"))
  ;[1 1 1] Get Score and Destroy Actor
  (bind _asrolling_ball_bp (cast `/Game/_RollingBall/Blueprints/RollingBallBP` OtherActor))
  (set `/Game/_RollingBall/Blueprints/RollingBallBP.Score` (+ (`/Game/_RollingBall/Blueprints/RollingBallBP.Score` _asrolling_ball_bp) (`self.Value`)) _asrolling_ball_bp)
  (bind _asobject_info (cast `/Game/_RollingBall/Blueprints/ObjectInfo` (`WidgetComponent.GetUserWidgetObject` (`self.Widget`))))
  (set `/Game/_RollingBall/Blueprints/ObjectInfo.Coin` self _asobject_info)
  (`KismetSystemLibrary.Delay` 0.2)
  (`self.K2_DestroyActor`))

(fn `UserConstructionScript`
  (`parent.UserConstructionScript`))