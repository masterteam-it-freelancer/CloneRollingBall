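; RollingBallBP is the player-controlled physics ball, rolled by movement input relative to the camera.
; Axis inputs apply acceleration-based torque to the mesh using control-rotation vectors, while look inputs steer controller pitch and yaw.
; Jump adds upward force behind a CanJump flag, which it sets back to true, so jumping never disables it.
; It also provides an IncrementScore function and quits the game on Escape.
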(event `self.ReceiveBeginPlay`)

(event `InputAxis|MoveFoward`
  (params (AxisValue :type "Float (single-precision)"))
  ;[1 1 1] MoveFoward
  (`PrimitiveComponent.AddTorqueInDegrees` (`self.StaticMesh`) (* (* (`KismetMathLibrary.GetRightVector` (`self.GetControlRotation`)) (`self.Add Torque`)) AxisValue) "None" true))

(event `InputAxis|RightFoward`
  (params (AxisValue :type "Float (single-precision)"))
  ;[1 1 1] MoveRightForward
  (`PrimitiveComponent.AddTorqueInDegrees` (`self.StaticMesh`) (* (`KismetMathLibrary.GetForwardVector` (`KismetMathLibrary.MakeRotator` 0.0 0.0 (.yaw (`self.GetControlRotation`)))) (* (`self.Add Torque`) AxisValue 1.0)) "None" true))

(event `InputAction|Jump`
  (params (Key :type "Key Structure"))
  ;[1 1 1] JumpFoward
  (:`Pressed`
    (if (`self.Can Jump`)
      (`PrimitiveComponent.AddForce` (`self.StaticMesh`) (`KismetMathLibrary.MakeVector` 0.0 0.0 (`self.JumpImpluse`)) "None" true)
      (set `self.Can Jump` true))))

(event `InputAxis|Lookup`
  (params (AxisValue :type "Float (single-precision)"))
  ;[1 1 1] Mouse Camera Control
  (`self.AddControllerPitchInput` (* AxisValue 1.0)))

(event `InputAxis|Turn`
  (params (AxisValue :type "Float (single-precision)"))
  ;[1 1 1] Mouse Camera Control
  (`self.AddControllerYawInput` (* AxisValue -1.0)))

(event `Key|Escape`
  (params (Key :type "Key Structure"))
  ;[1 1 1] Quit The Game
  (:`Pressed`
    (`KismetSystemLibrary.QuitGame` null "Quit")))

(fn `IncrementScore`
  (params (InSocre :type Integer))
  (set `self.Score` (+ (`self.Score`) InSocre)))

(fn `UserConstructionScript`)